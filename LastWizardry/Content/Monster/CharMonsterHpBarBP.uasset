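; CharMonsterHpBarBP is an actor that displays a monster's HP bar through its HpBar widget component.
; On BeginPlay it casts the component's widget to MonsterHpProgressBar and caches that widget's progress bar.
; UpdateLocation moves the actor to a given position without sweeping, and UpdateHpBar sets the bar's percent to Hp divided by MaxHp.
; It has no active Tick logic, so both position and health depend on calls to these functions.
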(event `self.ReceiveBeginPlay`
  (bind _asmonster_hp_progress_bar (cast `/Game/Monster/MonsterHpProgressBar` (`WidgetComponent.GetUserWidgetObject` (`self.HpBar`))))
  (set `self.ProgressBar_HpBar` (`/Game/Monster/MonsterHpProgressBar.ProgressBar_36` _asmonster_hp_progress_bar)))

(fn `UpdateHpBar`
  (params (Hp :type "Float (double-precision)") (MaxHp :type "Float (double-precision)"))
  (`ProgressBar.SetPercent` (`self.ProgressBar_HpBar`) (/ Hp MaxHp)))

(fn `UpdateLocation`
  (params (Location :type "Vector Structure"))
  (`self.K2_SetActorLocation` Location))

(fn `UserConstructionScript`)